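; BP_Hunter is the hunter character in DuckDuckKazoo, driven by an AI Blackboard.
; Each tick it sets an IsWalking flag from its horizontal movement speed.
; The HunterFleeing event sets IsFleeing and writes bIsFleeing to the Blackboard.
; IsFleeing resets on BeginPlay, and CheckRange is an empty stub.
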(event `self.ReceiveBeginPlay`
  (set `self.bIsFleeing` false))

(event `self.ReceiveTick`
  (params (DeltaSeconds :type "Float (single-precision)"))
  (`self.WalkingAnimation`))

(event `HunterFleeing`
  (set `self.bIsFleeing` true)
  (`BlackboardComponent.SetValueAsBool` (`AIBlueprintHelperLibrary.GetBlackboard` null) "bIsFleeing" true))

(fn `CheckRange`)

(fn `UserConstructionScript`)

(fn `WalkingAnimation`
  (if (> (`KismetMathLibrary.VSizeXY` (`MovementComponent.Velocity` (`self.CharacterMovement`))) 1.0)
    (set `self.bIsWalking` true)
    (else
      (set `self.bIsWalking` false))))