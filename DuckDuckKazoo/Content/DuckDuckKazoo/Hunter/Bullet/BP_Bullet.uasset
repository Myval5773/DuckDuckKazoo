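; BP_Bullet is the hunter's bullet in DuckDuckKazoo, which damages ducks it overlaps.
; When BulletCollision begins an overlap, it casts the other actor to BP_Duck and calls UpdateLifePoints if the duck's LifePoints are above zero.
; An AppliedDamage flag is set after a hit, so the next overlap only clears the flag and deals no damage.
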(event `self.BulletCollision.OnComponentBeginOverlap`
  (params (OverlappedComponent :type "PrimitiveComponent Object Reference") (OtherActor :type "Actor Object Reference") (OtherComp :type "PrimitiveComponent Object Reference") (OtherBodyIndex :type Integer) (bFromSweep :type Boolean) (SweepResult :type "HitResult Structure (by ref)"))
  (if (`self.bAppliedDamage`)
    (set `self.bAppliedDamage` false)
    (else
      (bind _asbp_duck (cast `/Game/DuckDuckKazoo/Duck/BP_Duck` OtherActor))
      (`/Engine/EditorBlueprintResources/StandardMacros.IsValid` _asbp_duck
        (:`Is Valid`
          (bind _output_get (set `self.Duck` _asbp_duck))
          (if (not (<= (`/Game/DuckDuckKazoo/Duck/BP_Duck.LifePoints` _output_get) 0))
            (`/Game/DuckDuckKazoo/Duck/BP_Duck.Update Life Points` (`self.Duck`))
            (set `self.bAppliedDamage` true)))))))

(fn `UserConstructionScript`)